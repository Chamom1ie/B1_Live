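; Player controller that lets the player switch possession between BP_B1Pawn actors in the level with number keys 1 to 4.
; BeginPlay caches every BP_B1Pawn in the Pawns array, and each key passes its number to PossessPlayer as a direct array index, leaving element 0 unreachable.
; PossessPlayer releases the current pawn before checking the index, so an invalid index leaves the controller without a pawn.
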(event `self.ReceiveBeginPlay`
  (bind _outactors (`GameplayStatics.GetAllActorsOfClass` "/Game/Blueprints/BP_B1Pawn.BP_B1Pawn_C"))
  (set `self.Pawns` _outactors))

(event `Key|One`
  (params (Key :type "Key Structure"))
  (:`Pressed`
    (`self.PossessPlayer` 1)))

(event `Key|Two`
  (params (Key :type "Key Structure"))
  (:`Pressed`
    (`self.PossessPlayer` 2)))

(event `Key|Three`
  (params (Key :type "Key Structure"))
  (:`Pressed`
    (`self.PossessPlayer` 3)))

(event `Key|Four`
  (params (Key :type "Key Structure"))
  (:`Pressed`
    (`self.PossessPlayer` 4)))

(fn `PossessPlayer`
  (params (Index :type Integer))
  (`self.UnPossess`)
  (if (`KismetArrayLibrary.Array_IsValidIndex` (`self.Pawns`) Index)
    (`self.Possess` (`|GetArrayItem` (`self.Pawns`) (`local.Index`)))))

(fn `UserConstructionScript`)