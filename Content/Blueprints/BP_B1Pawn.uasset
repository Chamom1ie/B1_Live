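; BP_B1Pawn is a player-controlled pawn with basic Enhanced Input movement, turning and a placeholder attack.
; On BeginPlay it adds IMC_Default to the player controller's input subsystem.
; IA_Move offsets the actor along its forward and right vectors and IA_Turn adds yaw, both by raw input values without delta-time scaling; movement does not sweep for collision.
; IA_Attack only prints a debug string.
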(event `self.ReceiveBeginPlay`
  (bind _asplayer_controller (cast `PlayerController` (`self.GetController`)))
  (message `EnhancedInputSubsystemInterface.AddMappingContext` (pcsubsystem `EnhancedInputLocalPlayerSubsystem` _asplayer_controller) "/Game/Input/IMC_Default.IMC_Default" 0 (struct)))

(event `EnhancedInput|/Game/Input/Actions/IA_Attack`
  (params (ActionValue :type Boolean) (ElapsedSeconds :type "Float (double-precision)") (TriggeredSeconds :type "Float (double-precision)") (InputAction :type "InputAction Object Reference" :default "/Game/Input/Actions/IA_Attack.IA_Attack"))
  (:`Triggered`
    (`KismetSystemLibrary.PrintString` "Hello")))

(event `EnhancedInput|/Game/Input/Actions/IA_Move`
  (params (ActionValue :type "Vector2D Structure") (ElapsedSeconds :type "Float (double-precision)") (TriggeredSeconds :type "Float (double-precision)") (InputAction :type "InputAction Object Reference" :default "/Game/Input/Actions/IA_Move.IA_Move"))
  (:`Triggered`
    (`self.K2_AddActorWorldOffset` (* (`self.GetActorForwardVector`) ActionValue_X))
    (`self.K2_AddActorWorldOffset` (* ActionValue_Y (`self.GetActorRightVector`)))))

(event `EnhancedInput|/Game/Input/Actions/IA_Turn`
  (params (ActionValue :type "Vector2D Structure") (ElapsedSeconds :type "Float (double-precision)") (TriggeredSeconds :type "Float (double-precision)") (InputAction :type "InputAction Object Reference" :default "/Game/Input/Actions/IA_Turn.IA_Turn"))
  (:`Triggered`
    (`self.K2_AddActorWorldRotation` (`KismetMathLibrary.MakeRotator` 0.0 0.0 ActionValue_X))))

(fn `UserConstructionScript`)